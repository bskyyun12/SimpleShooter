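; Ammo pickup that refills the player's current gun and respawns in place after a short delay.
; A Box overlap casts the other actor to BP_PlayerShooter and calls AddAmmo on its current gun with AmmoChargeAmount.
; Instead of being destroyed, the actor hides and disables Box collision, then a Delay restores visibility and query-only collision.
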(event `self.ReceiveActorBeginOverlap`
  (params (OtherActor :type "Actor Object Reference")))

(event `self.Box.OnComponentBeginOverlap`
  (params (OverlappedComponent :type "PrimitiveComponent Object Reference") (OtherActor :type "Actor Object Reference") (OtherComp :type "PrimitiveComponent Object Reference") (OtherBodyIndex :type Integer) (bFromSweep :type Boolean) (SweepResult :type "HitResult Structure (by ref)"))
  (bind _asbp_player_shooter (cast `/Game/BP_PlayerShooter` OtherActor))
  (`Gun.AddAmmo` (`ShooterCharacter.GetCurrentGun` _asbp_player_shooter) (`self.AmmoChargeAmount`))
  (`self.SetActorHiddenInGame` true)
  (`PrimitiveComponent.SetCollisionEnabled` (`self.Box`) "NoCollision")
  (`KismetSystemLibrary.Delay` 5.0)
  (`self.SetActorHiddenInGame` false)
  (`PrimitiveComponent.SetCollisionEnabled` (`self.Box`) "QueryOnly"))

(fn `UserConstructionScript`
  (`parent.UserConstructionScript`))